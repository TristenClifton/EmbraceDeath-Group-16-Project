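; Bat enemy that moves back and forth along the world X axis and can be killed by damage.
; Tick turns the actor to face its travel direction and adds movement input scaled by Speed.
; Hits against anything but the player pawn set the direction from the hit normal's X sign.
; Damage reduces Health, and at zero EnemyDied runs the parent logic, then destroys the actor.
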(event `self.ReceiveAnyDamage`
  (params (Damage :type "Float (single-precision)") (DamageType :type "DamageType Object Reference") (InstigatedBy :type "Controller Object Reference") (DamageCauser :type "Actor Object Reference"))
  (bind _output_get (set `self.Health` (- (`self.Health`) Damage)))
  (if (<= _output_get 0.0)
    (`self.EnemyDied`)))

(event `self.ReceiveBeginPlay`
  (set `self.Health` 100.0))

(event `self.ReceiveHit`
  (params (MyComp :type "PrimitiveComponent Object Reference") (Other :type "Actor Object Reference") (OtherComp :type "PrimitiveComponent Object Reference") (bSelfMoved :type Boolean) (HitLocation :type "Vector Structure") (HitNormal :type "Vector Structure") (NormalImpulse :type "Vector Structure") (Hit :type "HitResult Structure (by ref)"))
  ;[1 1 1] Don't change if coliding with player
  (if (not (== Other (`GameplayStatics.GetPlayerPawn` 0)))
    ;[1 1 1] Move in opposite direction of vector
    (set `self.MoveRight` (> (`KismetMathLibrary.BreakVector3f` HitNormal) 0.0))))

(event `self.ReceiveTick`
  (params (DeltaSeconds :type "Float (single-precision)"))
  (bind _speed (`self.Speed`))
  ;[1 1 1] Add Movement Based on MoveRight value
  (if (`self.MoveRight`)
    (`self.K2_SetActorRotation` (struct :`Yaw` 180.0))
    (`self.AddMovementInput` (1.0 0.0 0.0) _speed)
    (else
      (`self.K2_SetActorRotation` (struct))
      (`self.AddMovementInput` (1.0 0.0 0.0) (* _speed -1.0)))))

(fn `EnemyDied`
  (`parent.EnemyDied`)
  (`self.K2_DestroyActor`))

(fn `UserConstructionScript`
  (`parent.UserConstructionScript`))