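; Interactive vendor actor that tells players when they are at a shop.
; Overlap events cast to BP_PlayerBase, setting its AtVendor flag and VendorName from this actor's ShopName on entry.
; Leaving clears the flag and sets the name to the string "null".
; Interact only stores the passed player reference.
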(event `self.ReceiveActorBeginOverlap`
  (params (OtherActor :type "Actor Object Reference"))
  (bind _asbp_player_base (cast `/Game/Blueprints/BP_PlayerBase` OtherActor))
  (set `/Game/Blueprints/BP_PlayerBase.AtVendor` true _asbp_player_base)
  (set `/Game/Blueprints/BP_PlayerBase.VendorName` (`self.ShopName`) _asbp_player_base))

(event `self.ReceiveActorEndOverlap`
  (params (OtherActor :type "Actor Object Reference"))
  (bind _asbp_player_base (cast `/Game/Blueprints/BP_PlayerBase` OtherActor))
  (set `/Game/Blueprints/BP_PlayerBase.AtVendor` false _asbp_player_base)
  (set `/Game/Blueprints/BP_PlayerBase.VendorName` "null" _asbp_player_base))

(fn `Interact`
  (params (PlayerRef :type "/Game/Blueprints/BP_PlayerBase Object Reference"))
  (set `self.Player Ref` PlayerRef))

(fn `UserConstructionScript`
  (`parent.UserConstructionScript`))